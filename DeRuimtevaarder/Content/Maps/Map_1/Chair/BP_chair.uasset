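; Chair prop that briefly glitches into a wheelchair when anything overlaps its Col trigger.
; The overlap plays a glitch sound and swaps mesh visibility, then reverts with the same sound two seconds later.
; A parallel sequence branch plays a Robot voice line at the Robot's location five seconds after the overlap.
; HasGlitched blocks retriggering only during the swap, so the effect can repeat.
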(event OnComponentBeginOverlap(Col)
  (params (OverlappedComponent :type Primitive%20Component%20Object%20Reference) (OtherActor :type Actor%20Object%20Reference) (OtherComp :type Primitive%20Component%20Object%20Reference) (OtherBodyIndex :type Integer) (bFromSweep :type Boolean) (SweepResult :type Hit%20Result%20Structure%20%28by%20ref%29))
  ;[1 1 1] glitch => sound => glitch back => sound
  (if (not (Variables|Default|GethasGlitched))
    (Utilities|FlowControl|Sequence
      (:then_0
        (Variables|Default|SethasGlitched true)
        (Audio|PlaySoundatLocation "/Game/Maps/Map_1/Sounds/glitch.glitch" (Transformation|GetActorLocation) "0, 0, 0" 1.0 1.0 0.0 0 0 0)
        (Rendering|SetVisibility (Variables|Default|Getwheelchair) (Variables|Default|GetvisibilityTrue) false)
        (Rendering|SetVisibility (Variables|Default|Getchair) (Variables|Default|GetvisibilityFalse) false)
        (Utilities|FlowControl|Delay 2.0)
        (Audio|PlaySoundatLocation "/Game/Maps/Map_1/Sounds/glitch.glitch" (Transformation|GetActorLocation) "0, 0, 0" 1.0 1.0 0.0 0 0 0)
        (Rendering|SetVisibility (Variables|Default|Getchair) (Variables|Default|GetvisibilityTrue) false)
        (Rendering|SetVisibility (Variables|Default|Getwheelchair) (Variables|Default|GetvisibilityFalse) false)
        (Variables|Default|SethasGlitched false))
      (:then_1
        ;[1 1 1] Waarom kijk je zo vreemd?
        (Utilities|FlowControl|Delay 5.0)
        (Audio|PlaySoundatLocation "/Game/Maps/Map_1/Sounds/robot2.robot2" (Transformation|GetActorLocation (Variables|Default|Getrobot)) "0, 0, 0" 1.0 1.0 0.0 0 0 0)))))

(fn ConstructionScript)