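; BP_journal1 is a journal Actor that motion controllers can pick up and that plays its audio clip while held.
; Pickup, called by BP_MotionController, disables mesh physics, attaches the root to the given component and spawns the Journal1 sound at the actor's location.
; An AudioPlayed flag prevents repeat playback until Drop, which restores physics, detaches the actor, stops the sound and clears the flag.
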(event EventBeginPlay)

(event Collision|EventActorBeginOverlap
  (params (OtherActor :type Actor%20Object%20Reference)))

(event EventTick
  (params (DeltaSeconds :type Float%20%28single-precision%29)))

(event EventPickup
  (params (AttachTo :type Scene%20Component%20Object%20Reference))
  (Physics|SetSimulatePhysics (Variables|Debug|GetStaticMeshComponent) false)
  (Transformation|AttachComponentToComponent (VehicleSound|GetRootComponent) AttachTo "None" "KeepWorld" "KeepWorld" "KeepWorld" false)
  (if (not (Variables|Default|GetaudioPlayed))
    (bind _returnvalue (Audio|SpawnSoundatLocation "/Game/Maps/Map_1/Sounds/journal1.journal1" (Transformation|GetActorLocation) "0, 0, 0" 1.0 1.0 0.0 0 0))
    (Variables|Default|Set2dsound _returnvalue)
    (Variables|Default|SetaudioPlayed true)))

(event EventDrop
  (Physics|SetSimulatePhysics (Variables|Debug|GetStaticMeshComponent) true)
  (Transformation|DetachFromActor "KeepWorld" "KeepWorld" "KeepWorld")
  (Audio|Components|Audio|Stop (Variables|Default|Get2dsound))
  (Variables|Default|SetaudioPlayed false))

(fn ConstructionScript)