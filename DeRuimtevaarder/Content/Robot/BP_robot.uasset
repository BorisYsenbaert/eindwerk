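; BP_robot is a guide robot character that, once activated, moves to the player whenever pawn sensing spots them.
; On Map_1 it runs a delay-timed intro: it activates, plays voice lines, pulses talk and point animation flags, then enables player movement and shows the controls widget.
; On other levels it activates immediately.
; Tick sets the animation blueprint's walk flag from velocity.
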(event OnSeePawn(PawnSensing)
  (params (Pawn :type Pawn%20Object%20Reference))
  ;[1 1 1] AI
  (if (Variables|Default|GetactivateRobot)
    (bind _asplayer (Utilities|Casting|CastToPlayer Pawn))
    (AI|AIMoveTo self "0, 0, 0" _asplayer 3e+02 false)))

(event EventTick
  (params (DeltaSeconds :type Float%20%28single-precision%29))
  (bind _mesh (Variables|Character|GetMesh))
  (bind _returnvalue (Components|SkeletalMesh|GetAnimInstance _mesh))
  ;[1 1 1] Walk animation
  (if (!= (Math|Vector|VectorLength (Transformation|GetVelocity)) 0.0)
    (bind _asabp_robot (Utilities|Casting|CastToABP_robot _returnvalue))
    (Variables|/Game/Robot/Animations/ABP_robot.ABP_robot_C|SetcanWalk _asabp_robot true)
    (else
      (bind _asabp_robot_2 (Utilities|Casting|CastToABP_robot _returnvalue))
      (Variables|/Game/Robot/Animations/ABP_robot.ABP_robot_C|SetcanWalk _asabp_robot_2 false))))

(event EventBeginPlay
  (bind _returnvalue (Game|GetCurrentLevelName true))
  (if (Utilities|Enum|Equal(Enum) _returnvalue "Map_1")
    ;[1 1 1] Activate robot
    (Utilities|FlowControl|Delay 15.0)
    (Variables|Default|SetactivateRobot true)
    (Utilities|FlowControl|Delay 7.0)
    ;[1 1 1] Daar ben je! + test controls
    (Utilities|FlowControl|Sequence
      (:then_0
        (Audio|PlaySoundatLocation "/Game/Maps/Map_1/Sounds/robot1_1_Cue.robot1_1_Cue" (Transformation|GetActorLocation) "0, 0, 0" 1.0 1.0 0.0 0 0 0)
        (Utilities|FlowControl|Delay 4e+01)
        (bind _asplayer (Utilities|Casting|CastToPlayer (Game|GetPlayerCharacter 0)))
        (Utilities|FlowControl|Sequence
          (:then_0
            (Variables|/Game/VirtualRealityBP/Blueprints/Player.Player_C|SetcanMove _asplayer true))
          (:then_1
            (Rendering|SetVisibility (Variables|/Game/VirtualRealityBP/Blueprints/Player.Player_C|GetControllersWidget _asplayer) true false)
            ;[1 1 1] Klaar?
            (Utilities|FlowControl|Delay 3e+01)
            (Audio|PlaySoundatLocation "/Game/Maps/Map_1/Sounds/robot1_2_Cue.robot1_2_Cue" (Transformation|GetActorLocation) "0, 0, 0" 1.0 1.0 0.0 0 0 0))))
      (:then_1
        ;[1 1 1] Animation
        (Utilities|FlowControl|Delay 13.0)
        (bind _asabp_robot (Utilities|Casting|CastToABP_robot (Components|SkeletalMesh|GetAnimInstance (Variables|Character|GetMesh))))
        (Variables|/Game/Robot/Animations/ABP_robot.ABP_robot_C|Settalk _asabp_robot true)
        (Utilities|FlowControl|Delay 0.2)
        (Variables|/Game/Robot/Animations/ABP_robot.ABP_robot_C|Settalk _asabp_robot false)
        (Utilities|FlowControl|Delay 7.0)
        (bind _asabp_robot_2 (Utilities|Casting|CastToABP_robot (Components|SkeletalMesh|GetAnimInstance (Variables|Character|GetMesh))))
        (Variables|/Game/Robot/Animations/ABP_robot.ABP_robot_C|Setpoint _asabp_robot_2 true)
        (Utilities|FlowControl|Delay 0.2)
        (Variables|/Game/Robot/Animations/ABP_robot.ABP_robot_C|Setpoint _asabp_robot_2 false)
        (Utilities|FlowControl|Delay 8.0)
        (bind _asabp_robot_3 (Utilities|Casting|CastToABP_robot (Components|SkeletalMesh|GetAnimInstance (Variables|Character|GetMesh))))
        (Variables|/Game/Robot/Animations/ABP_robot.ABP_robot_C|Setpoint2 _asabp_robot_3 true)
        (Utilities|FlowControl|Delay 0.2)
        (Variables|/Game/Robot/Animations/ABP_robot.ABP_robot_C|Setpoint2 _asabp_robot_3 false)
        (Utilities|FlowControl|Delay 5.0)
        (bind _asabp_robot_4 (Utilities|Casting|CastToABP_robot (Components|SkeletalMesh|GetAnimInstance (Variables|Character|GetMesh))))
        (Variables|/Game/Robot/Animations/ABP_robot.ABP_robot_C|Settalk2 _asabp_robot_4 true)
        (Utilities|FlowControl|Delay 0.2)
        (Variables|/Game/Robot/Animations/ABP_robot.ABP_robot_C|Settalk2 _asabp_robot_4 false)))
    (else
      (Variables|Default|SetactivateRobot true))))

(fn ConstructionScript)